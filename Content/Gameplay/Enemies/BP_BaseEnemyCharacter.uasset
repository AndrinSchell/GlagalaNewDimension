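; Base enemy character that endlessly chases the player with a self-restarting AI MoveTo.
; An AttackCollision overlap with another I_Health actor starts a looping timer that deals Player-filtered damage until the overlap ends.
; Incoming damage and kills ignore Player and Destructable filters; damage updates the health bar widget or destroys the actor at zero health.
; The current and max health getters are stubs returning zero.
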(event OnComponentBeginOverlap(AttackCollision)
  (params (OverlappedComponent :type Primitive%20Component%20Object%20Reference) (OtherActor :type Actor%20Object%20Reference) (OtherComp :type Primitive%20Component%20Object%20Reference) (OtherBodyIndex :type Integer) (bFromSweep :type Boolean) (SweepResult :type Hit%20Result%20Structure%20%28by%20ref%29))
  ;[1 1 1] Handle Attacking
  (if (and (Utilities|DoesObjectImplementInterface OtherActor "/Script/GlagalaNewDimension.I_Health") (!= OtherActor self))
    (Variables|Default|SetAttackableActor OtherActor)
    (bind _returnvalue (Utilities|Time|SetTimerbyEvent (delegate Custom|Attack) (Variables|Default|GetAttackInterval) true))
    (Variables|Default|SetAttackTH _returnvalue)
    (CallFunction|Attack)))

(event OnComponentEndOverlap(AttackCollision)
  (params (OverlappedComponent :type Primitive%20Component%20Object%20Reference) (OtherActor :type Actor%20Object%20Reference) (OtherComp :type Primitive%20Component%20Object%20Reference) (OtherBodyIndex :type Integer))
  ;[1 1 1] Handle Attacking
  (if (== OtherActor (Variables|Default|GetAttackableActor))
    (Utilities|Time|ClearandInvalidateTimerbyHandle (Variables|Default|GetAttackTH))
    (Variables|Default|SetAttackableActor 0)))

(event Custom|ChasePlayer
  (AI|AIMoveTo self "0, 0, 0" (Game|GetPlayerCharacter 0) 5.0 true
    (:OnSuccess
      _)
    (:OnFail
      _))
  (CallFunction|ChasePlayer))

(event Custom|Attack
  ;[1 1 1] Handle Attacking
  (Utilities|IsValid (Variables|Default|GetAttackableActor)
    (:Is%20Valid
      (Class|IHealth|AddDamage(Message) (Variables|Default|GetAttackableActor) (Variables|Default|GetDamage) "Player" "Normal"))))

(event EventBeginPlay
  (Variables|Default|SetCurrentHealth (Variables|Default|GetMaxHealth))
  (EventDispatchers|BindEventtoHealthUpdated (EventDispatchers|CreateEvent :!event OnHealthUpdated))
  (Default|CallHealthUpdated (Variables|Default|GetCurrentHealth) (Variables|Default|GetMaxHealth))
  (CallFunction|ChasePlayer))

(event EventKill
  (params (Filter :type E_DamageFilter%20Enum :default "None"))
  ;[1 1 1] Death
  (if (and (Utilities|Enum|NotEqual(Enum) Filter "Destructable") (Utilities|Enum|NotEqual(Enum) Filter "Player"))
    (Actor|DestroyActor)))

(event EventAddDamage
  (params (Amount :type Float%20%28single-precision%29) (Filter :type E_DamageFilter%20Enum :default "None") (DamageType :type E_DamageType%20Enum :default "Normal"))
  ;[1 1 1] Damage
  (if (and (Utilities|Enum|NotEqual(Enum) Filter "Player") (Utilities|Enum|NotEqual(Enum) Filter "Destructable"))
    (if (<= (- (Variables|Default|GetCurrentHealth) Amount) 0.0)
      (Class|IHealth|Kill "None")
      (else
        (Variables|Default|SetCurrentHealth (- (Variables|Default|GetCurrentHealth) Amount))
        (Default|CallHealthUpdated (Variables|Default|GetCurrentHealth) (Variables|Default|GetMaxHealth))))))

(fn ConstructionScript)

(fn OnHealthUpdated
  (params (CurrentHealth :type Float%20%28double-precision%29) (MaxHealth :type Float%20%28double-precision%29))
  (Default|UpdateHealth (Variables|Default|GetWC_HealthBar) CurrentHealth MaxHealth))

(fn GetCurrentHealth
  (return 0.0))

(fn GetMaxHealth
  (return 0.0))