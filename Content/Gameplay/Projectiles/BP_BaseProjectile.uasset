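; Base projectile Actor that damages what it hits and destroys itself on impact.
; The construction script copies speed, gravity and homing settings into the projectile movement component.
; On a collision hit it calls ApplyImpactEffects, an empty hook here, then sends damage amount, filter and type to actors implementing I_Health.
; The projectile is destroyed whether or not the hit actor takes damage.
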(event OnComponentHit(Collision)
  (params (HitComponent :type Primitive%20Component%20Object%20Reference) (OtherActor :type Actor%20Object%20Reference) (OtherComp :type Primitive%20Component%20Object%20Reference) (NormalImpulse :type Vector :default "0, 0, 0") (Hit :type Hit%20Result%20Structure%20%28by%20ref%29))
  (CallFunction|ApplyImpactEffects Hit)
  (if (Utilities|DoesObjectImplementInterface OtherActor "/Script/GlagalaNewDimension.I_Health")
    (Class|IHealth|AddDamage(Message) OtherActor (Variables|Damage|GetDamage) (Variables|Damage|GetDamageFilter) (Variables|Damage|GetDamageType))
    (Actor|DestroyActor)
    (else
      (Actor|DestroyActor))))

(event Custom|ApplyImpactEffects
  (params (Hit :type Hit%20Result%20Structure)))

(event EventBeginPlay)

(event Collision|EventActorBeginOverlap
  (params (OtherActor :type Actor%20Object%20Reference)))

(event EventTick
  (params (DeltaSeconds :type Float%20%28single-precision%29)))

(fn ConstructionScript
  (bind _speed (Variables|Movement|GetSpeed))
  (Variables|/Script/Engine.ProjectileMovementComponent|SetInitialSpeed (Variables|Default|GetProjectileMovementComp) _speed)
  (Variables|/Script/Engine.ProjectileMovementComponent|SetMaxSpeed (Variables|Default|GetProjectileMovementComp) _speed)
  (Variables|/Script/Engine.ProjectileMovementComponent|SetProjectileGravityScale (Variables|Default|GetProjectileMovementComp) (Variables|Movement|GetGravity))
  (Variables|/Script/Engine.ProjectileMovementComponent|SetbIsHomingProjectile (Variables|Default|GetProjectileMovementComp) (Variables|Default|GetIsHoming)))