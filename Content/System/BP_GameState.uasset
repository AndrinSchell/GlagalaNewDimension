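; Game state Blueprint that owns the in-game menu, pausing and the game timer.
; Shortly after BeginPlay it caches the player character (after a placeholder delay), creates the menu widget, binds its start and continue events, and opens it with the game paused.
; Pausing also toggles the mouse cursor and menu visibility.
; Starting the game unpauses and runs a looping timer for game time, announcing timer state changes through a dispatcher.
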(event Custom|StartGameClicked
  ;[1 1 1] IngameMenu
  (CallFunction|PauseGame false)
  (CallFunction|SetTmerEnabled true))

(event Custom|InitIngameMenu
  ;[1 1 1] IngameMenu
  (bind _returnvalue (UserInterface|CreateWidget "/Game/System/UI/IngameMenu/WBP_IngameMenu.WBP_IngameMenu_C" (Game|GetPlayerController 0)))
  (Variables|Default|SetWBP_IngameMenu _returnvalue)
  (Default|InitWIdget (Variables|Default|GetWBP_IngameMenu))
  (CallFunction|BindIngameMenuEvents)
  (CallFunction|PauseGame true)
  (Default|SetActiveMenu (Variables|Default|GetWBP_IngameMenu) "NewEnumerator0"))

(event Custom|ToggleGamePaused
  (CallFunction|PauseGame (not (Game|IsGamePaused)))
  (Default|SetActiveMenu (Variables|Default|GetWBP_IngameMenu) "NewEnumerator1"))

(event EventBeginPlay
  ;[1 1 1] Begin Play
  (Utilities|FlowControl|Delay 0.2)
  (Utilities|FlowControl|Sequence
    (:then_0
      ;;[1 0 0] Replace with waiting func!
      (bind _returnvalue (Actor|GetActorOfClass "/Game/System/Player/BP_PlayerCharacter.BP_PlayerCharacter_C"))
      (Variables|Default|SetPlayerCharacterRef _returnvalue))
    (:then_1
      (CallFunction|InitIngameMenu))))

(fn ConstructionScript)

(fn SetTmerEnabled
  (params (Enabled :type Boolean))
  (if Enabled
    (bind _returnvalue (Utilities|Time|SetTimerbyEvent (EventDispatchers|CreateEvent :!event IncreaseGameTime) (Variables|Default|GetTimerAccuracy) true))
    (Variables|Default|SetGameTimerTH _returnvalue)
    (Default|CallGameTimerEnabledChanged true (Variables|Default|GetTimerAccuracy))
    (else
      (Utilities|Time|ClearandInvalidateTimerbyHandle (Variables|Default|GetGameTimerTH))
      (Default|CallGameTimerEnabledChanged false 0.0))))

(fn IncreaseGameTime
  (Variables|Default|SetGameTime (+ (Variables|Default|GetTimerAccuracy) (Variables|Default|GetGameTime))))

(fn PauseGame
  (params (Pause :type Boolean))
  (Game|SetGamePaused Pause)
  (Variables|/Script/Engine.PlayerController|SetbShowMouseCursor (Game|GetPlayerController 0) Pause)
  (if Pause
    (UserInterface|Viewport|AddtoViewport (Variables|Default|GetWBP_IngameMenu) 0)
    (else
      (Widget|RemovefromParent (Variables|Default|GetWBP_IngameMenu)))))

(fn BindIngameMenuEvents
  (Utilities|FlowControl|Sequence
    (:then_0
      (EventDispatchers|BindEventtoOnStartGameClicked (Variables|Default|GetWBP_IngameMenu) (EventDispatchers|CreateEvent :!event Custom|StartGameClicked)))
    (:then_1
      (EventDispatchers|BindEventtoOnContinueGameClicked (Variables|Default|GetWBP_IngameMenu) (EventDispatchers|CreateEvent :!event Custom|ToggleGamePaused)))))