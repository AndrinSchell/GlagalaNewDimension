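; Blueprint function library that turns a game time in seconds into display text.
; GametimeToText splits the time into minutes, seconds and hundredths of a second (labeled milsec) using division with remainder, then joins them with colons.
; MakeTwoDigitNumber pads each part, prefixing a zero to values of nine or less.
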(fn GametimetoText
  (params (GameTime :type Float%20%28double-precision%29))
  (return (Utilities|Text|FormatText "{min}:{sec}:{milsec}" (CallFunction|MakeTwoDigitNumber (.ReturnValue (Math|Float|Division(WholeandRemainder) GameTime 6e+01))) (CallFunction|MakeTwoDigitNumber (Math|Float|Truncate (.Remainder (Math|Float|Division(WholeandRemainder) GameTime 6e+01)))) (CallFunction|MakeTwoDigitNumber (Math|Float|Truncate (* (.Remainder (Math|Float|Division(WholeandRemainder) GameTime 1.0)) 1e+02))))))

(fn MakeTwoDigitNumber
  (params (Number :type Integer))
  (return (Utilities|String|SelectText (Utilities|Text|FormatText "0{val}" Number) (Utilities|Text|ToText(Integer) Number) (<= Number 9))))