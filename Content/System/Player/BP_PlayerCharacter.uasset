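; Player character Blueprint that tracks health and restarts the game level on death.
; AddDamage subtracts health and calls a health-updated notification, while lethal damage calls Kill, whose Respawn opens BasicLevel without updating health.
; GetCurrentHealth and GetMaxHealth are stubs returning zero.
; Tick draws long-lived debug points at the mesh location, tracing the player's path.
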(event EventBeginPlay)

(event EventKill
  (params (Filter :type E_DamageFilter%20Enum :default "None"))
  ;[1 1 1] Health
  (CallFunction|Respawn))

(event EventAddDamage
  (params (Amount :type Float%20%28single-precision%29) (Filter :type E_DamageFilter%20Enum :default "None") (DamageType :type E_DamageType%20Enum :default "Normal"))
  ;[1 1 1] Health
  (if (<= (- (Variables|Default|GetCurrentHealth) Amount) 0.0)
    (Class|IHealth|Kill "None")
    (else
      (Variables|Default|SetCurrentHealth (- (Variables|Default|GetCurrentHealth) Amount))
      (Default|CallHealthUpdated (Variables|Default|GetCurrentHealth) (Variables|Default|GetMaxHealth)))))

(event EventTick
  (params (DeltaSeconds :type Float%20%28single-precision%29))
  (Rendering|Debug|DrawDebugPoint (Transformation|GetWorldLocation (Variables|Character|GetMesh)) 1e+01 "(R=1.000000,G=0.069903,B=0.000000,A=1.000000)" 2e+01))

(fn ConstructionScript)

(fn Respawn
  (Game|OpenLevel(byObjectReference) "/Game/Levels/TestLevels/BasicLevel.BasicLevel"))

(fn GetCurrentHealth
  (return 0.0))

(fn GetMaxHealth
  (return 0.0))